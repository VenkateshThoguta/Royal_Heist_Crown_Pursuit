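; Key pickup Blueprint that the player collects by pressing K while standing inside its Box trigger.
; Overlap by the ThirdPersonCharacter enables input on the actor and opens a Gate; leaving disables input and closes it.
; A K press through the open Gate plays an inspect-item sound, sets the character's Key flag to true and destroys the key.
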(event OnComponentBeginOverlap(Box)
  (params (OverlappedComponent :type Primitive%20Component%20Object%20Reference) (OtherActor :type Actor%20Object%20Reference) (OtherComp :type Primitive%20Component%20Object%20Reference) (OtherBodyIndex :type Integer) (bFromSweep :type Boolean) (SweepResult :type Hit%20Result%20Structure%20%28by%20ref%29))
  (bind _asthird_person_character (Utilities|Casting|CastToThirdPersonCharacter OtherActor))
  (Input|EnableInput (Game|GetPlayerController 0))
  (Utilities|FlowControl|Gate true) ; enters at Open
)

(event OnComponentEndOverlap(Box)
  (params (OverlappedComponent :type Primitive%20Component%20Object%20Reference) (OtherActor :type Actor%20Object%20Reference) (OtherComp :type Primitive%20Component%20Object%20Reference) (OtherBodyIndex :type Integer))
  (Utilities|Casting|CastToThirdPersonCharacter OtherActor)
  (Input|DisableInput (Game|GetPlayerController 0))
  (Utilities|FlowControl|Gate true) ; enters at Close
)

(event Input|KeyboardEvents|K
  (params (Key :type Key%20Structure :default "None"))
  (:Pressed
    (Utilities|FlowControl|Gate true
      (:Exit
        (Audio|PlaySoundatLocation "/Game/Level1Assests/Level2_Door/Door_Assets/422709__niamhd00145229__inspect-item.422709__niamhd00145229__inspect-item" (Transformation|GetActorLocation) "0, 0, 0" 1.0 1.0 0.0 0 0 0)
        (Variables|/Game/ThirdPersonCPP/Blueprints/ThirdPersonCharacter.ThirdPersonCharacter_C|Setkey (stale OnComponentBeginOverlap(Box) _asthird_person_character) true)
        (Actor|DestroyActor)))))

(fn ConstructionScript)