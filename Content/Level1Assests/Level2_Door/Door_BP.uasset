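; Door actor that the player swings open or closed by pressing E while standing in its trigger box.
; Box overlap with the ThirdPersonCharacter enables input and opens a gate, and leaving reverses both.
; E plays a metal door sound, then flip-flops a timeline that lerps the mesh's yaw between closed and open angles.
; An unconnected key check and locked sound never run.
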(event OnComponentBeginOverlap(Box)
  (params (OverlappedComponent :type Primitive%20Component%20Object%20Reference) (OtherActor :type Actor%20Object%20Reference) (OtherComp :type Primitive%20Component%20Object%20Reference) (OtherBodyIndex :type Integer) (bFromSweep :type Boolean) (SweepResult :type Hit%20Result%20Structure%20%28by%20ref%29))
  (Utilities|Casting|CastToThirdPersonCharacter OtherActor)
  (Input|EnableInput (Game|GetPlayerController 0))
  (Utilities|FlowControl|Gate true) ; enters at Open
)

(event OnComponentEndOverlap(Box)
  (params (OverlappedComponent :type Primitive%20Component%20Object%20Reference) (OtherActor :type Actor%20Object%20Reference) (OtherComp :type Primitive%20Component%20Object%20Reference) (OtherBodyIndex :type Integer))
  (Utilities|Casting|CastToThirdPersonCharacter OtherActor)
  (Input|DisableInput (Game|GetPlayerController 0))
  (Utilities|FlowControl|Gate true) ; enters at Close
)

(event EventBeginPlay)

(event Collision|EventActorBeginOverlap
  (params (OtherActor :type Actor%20Object%20Reference)))

(event EventTick
  (params (DeltaSeconds :type Float%20%28single-precision%29)))

(event Input|KeyboardEvents|E
  (params (Key :type Key%20Structure :default "None"))
  (:Pressed
    (Audio|PlaySoundatLocation "/Game/Level1Assests/Level2_Door/Door_Assets/422682__niamhd00145229__metal-door.422682__niamhd00145229__metal-door" (Transformation|GetActorLocation) "0, 0, 0" 1.0 1.0 0.0 0 0 0)
    (Utilities|FlowControl|Gate true
      (:Exit
        (Utilities|FlowControl|FlipFlop
          (:A
            (bind _newtrack_0 (Timeline|open/close Play)
              (:Update
                (Transformation|SetRelativeRotation (Variables|Default|GetStaticMesh) (Math|Rotator|MakeRotator 0.0 0.0 (Math|Float|Lerp (Variables|Default|Getcloseangle) (Variables|Default|Getopenangle) _newtrack_0)) false false))))
          (:B
            (Timeline|open/close Reverse)))))))

(fn ConstructionScript)